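; Player character Blueprint for third-person movement, camera look and rifle combat, driven by Enhanced Input.
; Equipping toggles rifle visibility after a short delay, and aiming plays a timeline that shortens and raises the spring arm.
; Holding fire with the rifle equipped loops a timer that plays the firing montage.
; Its notify line-traces from the muzzle, spawning impact sparks, muzzle flash and camera shake, without applying damage.
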(event Custom|Fire%20Rifle
  (bind _rifle (Variables|Default|GetRifle))
  (bind _rifle_2 (Variables|Default|GetRifle))
  (bind _returnvalue (Transformation|GetSocketTransform _rifle_2 "Muzzle" "RTS_World"))
  (bind _returnvalue_2 (Transformation|GetSocketTransform _rifle "Muzzle" "RTS_World"))
  (Animation|Montage|PlayMontage (Variables|Character|GetMesh) "/Game/Characters/Animation/Rifles/Fire_Rifle_Ironsights_Montage.Fire_Rifle_Ironsights_Montage"
    (:OnNotifyBegin
      (Utilities|FlowControl|Sequence
        (:then_0
          (bind (_outhit _returnvalue_3) (Collision|LineTraceByChannel (.location _returnvalue_2) (+ (.location _returnvalue_2) (* (Math|Vector|GetForwardVector (.rotation _returnvalue_2)) 5e+03)) "TraceTypeQuery1" false 0 "None"))
          (if _returnvalue_3
            (Effects|SpawnEmitteratLocation "/Game/InfinityBladeEffects/Effects/FX_Combat_Base/Impact/P_ImpactSpark.P_ImpactSpark" (.ImpactPoint (Collision|BreakHitResult _outhit)) (Math|Rotator|MakeRotfromX (.Normal (Collision|BreakHitResult _outhit))) "0.300000,0.300000,0.300000" true "AutoRelease")))
        (:then_1
          (Effects|SpawnEmitterAttached "/Game/InfinityBladeEffects/Effects/FX_Mobile/Fire/combat/P_FireBall_Strong_MuzzFlash_01.P_FireBall_Strong_MuzzFlash_01" (Variables|Default|GetRifle) "Muzzle" (.location _returnvalue) (.rotation _returnvalue) "0.200000,0.200000,0.200000" "KeepWorldPosition" true "AutoRelease")
          (Camera|PlayWorldCameraShake "/Game/Blueprints/BP_RifleCameraShake.BP_RifleCameraShake_C" (Transformation|GetActorLocation) 0.0 5e+02))))))

(event Input|EnhancedActionEvents|EnhancedInputActionIA_Move
  (params (ActionValue :type Vector%202D%20Structure) (ElapsedSeconds :type Float%20%28double-precision%29) (TriggeredSeconds :type Float%20%28double-precision%29) (InputAction :type Input%20Action%20Object%20Reference :default "/Game/Input/IA_Move.IA_Move"))
  (bind _returnvalue (Pawn|GetControlRotation :!class /Script/Engine.Pawn))
  (bind _returnvalue_2 (Pawn|GetControlRotation :!class /Script/Engine.Pawn))
  ;[0.1458 0.1458 0.1458] Movement and Camera Look
  (Pawn|Input|AddMovementInput (Math|Vector|GetRightVector (Math|Rotator|MakeRotator (.roll _returnvalue) 0.0 (.yaw _returnvalue))) (.x ActionValue) false)
  (Pawn|Input|AddMovementInput (Math|Vector|GetForwardVector (Math|Rotator|MakeRotator (.roll _returnvalue_2) 0.0 (.yaw _returnvalue_2))) (.y ActionValue) false))

(event Input|EnhancedActionEvents|EnhancedInputActionIA_Look
  (params (ActionValue :type Vector%202D%20Structure) (ElapsedSeconds :type Float%20%28double-precision%29) (TriggeredSeconds :type Float%20%28double-precision%29) (InputAction :type Input%20Action%20Object%20Reference :default "/Game/Input/IA_Look.IA_Look"))
  ;[0.1458 0.1458 0.1458] Movement and Camera Look
  (Pawn|Input|AddControllerYawInput (.x ActionValue))
  (Pawn|Input|AddControllerPitchInput (* (.y ActionValue) -1.0)))

(event Input|EnhancedActionEvents|EnhancedInputActionIA_EquipRifle
  (params (ActionValue :type Boolean) (ElapsedSeconds :type Float%20%28double-precision%29) (TriggeredSeconds :type Float%20%28double-precision%29) (InputAction :type Input%20Action%20Object%20Reference :default "/Game/Input/IA_EquipRifle.IA_EquipRifle"))
  ;[0.1458 0.1458 0.1458] Equip and Unequip Riffle
  (:Started
    (if (not (Variables|Default|GetRifleEquipped))
      (Variables|Default|SetRifleEquipped true)
      (Utilities|FlowControl|Delay 0.5)
      (Rendering|SetVisibility (Variables|Default|GetRifle) true false)
      (else
        (Variables|Default|SetRifleEquipped false)
        (Utilities|FlowControl|Delay 0.8)
        (Rendering|SetVisibility (Variables|Default|GetRifle) false false)))))

(event Input|EnhancedActionEvents|EnhancedInputActionIA_Aim
  (params (ActionValue :type Boolean) (ElapsedSeconds :type Float%20%28double-precision%29) (TriggeredSeconds :type Float%20%28double-precision%29) (InputAction :type Input%20Action%20Object%20Reference :default "/Game/Input/IA_Aim.IA_Aim"))
  (bind _springarm (Variables|Default|GetSpringArm))
  ;[0.1458 0.1458 0.1458] Aiming
  (:Started
    (Variables|Default|SetIs%20Aiming true)
    (bind _arm_length (Timeline|Aim Play)
      (:Update
        (Variables|/Script/Engine.SpringArmComponent|SetTargetArmLength (Variables|Default|GetSpringArm) (Math|Float|Lerp 3e+02 1.5e+02 _arm_length))
        (Variables|/Script/Engine.SpringArmComponent|SetSocketOffset _springarm (Math|Vector|MakeVector (.x (Variables|/Script/Engine.SpringArmComponent|GetSocketOffset _springarm)) (.y (Variables|/Script/Engine.SpringArmComponent|GetSocketOffset _springarm)) (Math|Float|Lerp 0.0 25.0 _arm_length))))))
  (:Completed
    (Variables|Default|SetIs%20Aiming false)
    (Timeline|Aim Reverse)))

(event Input|EnhancedActionEvents|EnhancedInputActionIA_Fire
  (params (ActionValue :type Boolean) (ElapsedSeconds :type Float%20%28double-precision%29) (TriggeredSeconds :type Float%20%28double-precision%29) (InputAction :type Input%20Action%20Object%20Reference :default "/Game/Input/IA_Fire.IA_Fire"))
  (:Started
    (if (Variables|Default|GetRifleEquipped)
      (bind _returnvalue (Utilities|Time|SetTimerbyEvent (delegate Custom|Fire%20Rifle) 0.1 true))))
  (:Completed
    (Utilities|Time|ClearandInvalidateTimerbyHandle _returnvalue)))

(event EventBeginPlay
  ;[0.1458 0.1458 0.1458] Add Input
  (Input|AddMappingContext (PlayerController|LocalPlayerSubsystems|GetEnhancedInputLocalPlayerSubsystem (Game|GetPlayerController 0)) "/Game/Input/IMC_PlayerInput.IMC_PlayerInput" 0 "(bIgnoreAllPressedKeysUntilRelease=True,bForceImmediately=False,bNotifyUserSettings=False)"))

(fn ConstructionScript)